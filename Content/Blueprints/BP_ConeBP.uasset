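; BP_ConeBP is an actor that bobs vertically between its starting height and a point Max units above it.
; BeginPlay records the starting Z as the lower bound and derives the upper bound from it.
; Tick moves the Z value at Speed scaled by delta time, sets the location without sweep, and reverses direction once either bound is passed.
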(event EventBeginPlay
  (bind _returnvalue (Transformation|GetActorLocation))
  (Variables|Default|SetbIsUp true)
  (Variables|Default|SetCurrentZValue (.z _returnvalue))
  (Variables|Default|SetMinHeight (.z _returnvalue))
  (Variables|Default|SetMaxHeight (+ (.z _returnvalue) (Variables|Default|GetMax))))

(event EventTick
  (params (DeltaSeconds :type Float%20%28single-precision%29))
  (bind _returnvalue (Transformation|GetActorLocation))
  (bind _speed (Variables|Default|GetSpeed))
  (bind _returnvalue_2 (* DeltaSeconds _speed))
  (if (Variables|Default|GetbIsUp)
    (Variables|Default|SetCurrentZValue (+ (Variables|Default|GetCurrentZValue) _returnvalue_2))
    (else
      (Variables|Default|SetCurrentZValue (- (Variables|Default|GetCurrentZValue) _returnvalue_2))))
  (Transformation|SetActorLocation (Math|Vector|MakeVector (.x _returnvalue) (.y _returnvalue) (Variables|Default|GetCurrentZValue)) false false)
  (if (> (Variables|Default|GetCurrentZValue) (Variables|Default|GetMaxHeight))
    (Variables|Default|SetbIsUp false))
  (if (< (Variables|Default|GetCurrentZValue) (Variables|Default|GetMinHeight))
    (Variables|Default|SetbIsUp true)))

(fn ConstructionScript)